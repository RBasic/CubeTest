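; Door puzzle actor where a cube is pushed onto a target to open a door.
; ImpulseComponent pushes the cube away from the given actor, only while that actor's FloatingPawnMovement has velocity.
; When the cube hits Target, Solved is set and each hit event moves cube and door one VInterpTo step toward target and open position, with no Tick or timeline.
; ResetCubeLocation restores the position saved at BeginPlay.
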(event `self.ReceiveBeginPlay`
  (set `self.CubeInitialLocation` (`SceneComponent.K2_GetComponentLocation` (`self.Cube`))))

(event `/Game/Blueprints/Interfaces/PhysicalAssetWithPawnMovement.ImpulseComponent`
  (params (actor :type "/Game/Blueprints/Player/BP_BasePlayer Object Reference") (component :type "StaticMeshComponent Object Reference") (force :type "Float (single-precision)"))
  (bind _returnvalue (`SceneComponent.K2_GetComponentLocation` component))
  (if (== component (`self.Cube`))
    (`PrimitiveComponent.AddImpulse` component (- (+ _returnvalue (* (- _returnvalue (`self.K2_GetActorLocation` actor)) (* (`KismetMathLibrary.VSize` (`KismetMathLibrary.Normal` (`MovementComponent.Velocity` (`/Game/Blueprints/Player/BP_BasePlayer.FloatingPawnMovement` actor)))) force))) _returnvalue) "None" false)))

(event `self.Target.OnComponentHit`
  (params (HitComponent :type "PrimitiveComponent Object Reference") (OtherActor :type "Actor Object Reference") (OtherComp :type "PrimitiveComponent Object Reference") (NormalImpulse :type "Vector Structure") (Hit :type "HitResult Structure (by ref)"))
  (bind _cube (`self.Cube`))
  (bind _door (`self.Door`))
  (bind _returnvalue (`SceneComponent.K2_GetComponentLocation` _cube))
  (if (== OtherComp _cube)
    (set `self.bSolved` true)
    (`SceneComponent.K2_SetWorldLocation` (`self.Cube`) (`KismetMathLibrary.VInterpTo` _returnvalue (`KismetMathLibrary.MakeVector` (.x (`SceneComponent.K2_GetComponentLocation` (`self.Target`))) (.y (`SceneComponent.K2_GetComponentLocation` (`self.Target`))) (.z _returnvalue)) (`GameplayStatics.GetWorldDeltaSeconds`) 1.0) false false)
    (`SceneComponent.K2_SetRelativeLocation` _door (`KismetMathLibrary.VInterpTo` (`SceneComponent.RelativeLocation` _door) (`self.doorOpenLocation`) (`GameplayStatics.GetWorldDeltaSeconds`) 1.0) false false)))

(fn `ResetCubeLocation`
  (`SceneComponent.K2_SetWorldLocation` (`self.Cube`) (`self.CubeInitialLocation`) false false))

(fn `UserConstructionScript`)