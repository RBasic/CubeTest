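; BP_PlatformEnigma is a level-design platform, apparently for puzzles, that slides between an on and an off position.
; A timeline scales RelativeMovement to set the Platform's relative location, playing forward when switched off and in reverse when switched on.
; ResetPlatform, also run at BeginPlay, applies the ShouldBeOn state, while TogglePlatform flips the current IsOn state.
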(event `self.ReceiveBeginPlay`
  (`self.ResetPlatform`))

(event `ResetPlatform`
  (if (`self.shouldBeOn`)
    (set `self.isOn` true :!label _label)
    (bind (_direction _factor) (`Timeline|AnimatePlatform` :!via `Reverse` :!label _label_2)
      (:`Update`
        (`SceneComponent.K2_SetRelativeLocation` (`self.Platform`) (* (`self.RelativeMovement`) _factor) false false)))
    (else
      (set `self.isOn` false :!label _label_3)
      (goto _label_2))))

(event `TogglePlatform`
  (if (`self.isOn`)
    (goto _label_3)
    (else
      (goto _label))))

(fn `UserConstructionScript`)