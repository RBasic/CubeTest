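; BP_GrabEnigma is a grab puzzle where the player brings a cube to a target to open a door.
; Inside the Box trigger, BP_BasePlayer gets input, and Grab toggles the cube between attachment to the player's GrabPoint and physics simulation.
; A cube hit on Target sets Solved, blocking further grab toggles, and nudges cube and door with one VInterpTo step per hit.
; ResetCubeLocation restores the cube's BeginPlay position.
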(event `self.ReceiveBeginPlay`
  (set `self.CubeInitialLocation` (`SceneComponent.K2_GetComponentLocation` (`self.Cube`))))

(event `self.Target.OnComponentHit`
  (params (HitComponent :type "PrimitiveComponent Object Reference") (OtherActor :type "Actor Object Reference") (OtherComp :type "PrimitiveComponent Object Reference") (NormalImpulse :type "Vector Structure") (Hit :type "HitResult Structure (by ref)"))
  (bind _cube (`self.Cube`))
  (bind _door (`self.Door`))
  (bind _returnvalue (`SceneComponent.K2_GetComponentLocation` _cube))
  (if (== OtherComp _cube)
    (set `self.bSolved` true)
    (`SceneComponent.K2_SetWorldLocation` (`self.Cube`) (`KismetMathLibrary.VInterpTo` _returnvalue (`KismetMathLibrary.MakeVector` (.x (`SceneComponent.K2_GetComponentLocation` (`self.Target`))) (.y (`SceneComponent.K2_GetComponentLocation` (`self.Target`))) (.z _returnvalue)) (`GameplayStatics.GetWorldDeltaSeconds`) 1.0) false false)
    (`SceneComponent.K2_SetRelativeLocation` _door (`KismetMathLibrary.VInterpTo` (`SceneComponent.RelativeLocation` _door) (`self.doorOpenLocation`) (`GameplayStatics.GetWorldDeltaSeconds`) 1.0) false false)))

(event `self.Box.OnComponentBeginOverlap`
  (params (OverlappedComponent :type "PrimitiveComponent Object Reference") (OtherActor :type "Actor Object Reference") (OtherComp :type "PrimitiveComponent Object Reference") (OtherBodyIndex :type Integer) (bFromSweep :type Boolean) (SweepResult :type "HitResult Structure (by ref)"))
  (bind _asbp_base_player (cast `/Game/Blueprints/Player/BP_BasePlayer` OtherActor))
  (set `self.PlayerRef` _asbp_base_player)
  (`self.EnableInput` (`GameplayStatics.GetPlayerController` 0)))

(event `self.Box.OnComponentEndOverlap`
  (params (OverlappedComponent :type "PrimitiveComponent Object Reference") (OtherActor :type "Actor Object Reference") (OtherComp :type "PrimitiveComponent Object Reference") (OtherBodyIndex :type Integer))
  (cast `/Game/Blueprints/Player/BP_BasePlayer` OtherActor)
  (set `self.PlayerRef` null)
  (`self.DisableInput` (`GameplayStatics.GetPlayerController` 0)))

(event `InputAction|Grab`
  (params (Key :type "Key Structure"))
  (bind _cube (`self.Cube`))
  (:`Pressed`
    (bind _playerref (`self.PlayerRef`)
      (:`then`
        (if (not (`self.bSolved`))
          (if (`self.bGrabbed`)
            (set `self.bGrabbed` false)
            (`SceneComponent.K2_DetachFromComponent` _cube "KeepWorld" "KeepWorld" "KeepWorld" true)
            (`PrimitiveComponent.SetSimulatePhysics` _cube true)
            (else
              (set `self.bGrabbed` true)
              (`PrimitiveComponent.SetSimulatePhysics` _cube false)
              (`SceneComponent.K2_AttachToComponent` _cube (`/Game/Blueprints/Player/BP_BasePlayer.GrabPoint` _playerref) "None" "SnapToTarget" "SnapToTarget" "KeepRelative" true)))))
      (:`else`))))

(fn `ResetCubeLocation`
  (`SceneComponent.K2_SetWorldLocation` (`self.Cube`) (`self.CubeInitialLocation`) false false))

(fn `UserConstructionScript`)