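; BP_Checkpoint is a level checkpoint that restores a player's health and records their respawn point when they enter its box trigger.
; On overlap, it sets the BP_BasePlayer's Health and saves that player's current transform, rather than its own, as LastCheckpoint.
; A stored player reference skips repeat overlaps by the same player.
; The ActivateCheckpoint timeline then animates the Plane's Color and EmissiveColor material parameters to show activation.
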(event `self.Box.OnComponentBeginOverlap`
  (params (OverlappedComponent :type "PrimitiveComponent Object Reference") (OtherActor :type "Actor Object Reference") (OtherComp :type "PrimitiveComponent Object Reference") (OtherBodyIndex :type Integer) (bFromSweep :type Boolean) (SweepResult :type "HitResult Structure (by ref)"))
  (bind _plane (`self.Plane`))
  (bind _asbp_base_player (cast `/Game/Blueprints/Player/BP_BasePlayer` OtherActor))
  (if (!= _asbp_base_player (`self.PlayerRef`))
    (set `/Game/Blueprints/Player/BP_BasePlayer.Health` 3 _asbp_base_player)
    (set `self.PlayerRef` _asbp_base_player)
    (set `/Game/Blueprints/Player/BP_BasePlayer.lastCheckpoint` (`self.GetTransform` _asbp_base_player) _asbp_base_player)
    (bind (_direction _checkpointcolor) (`Timeline|activateCheckpoint` :!via `PlayFromStart`)
      (:`Update`
        (`MeshComponent.SetVectorParameterValueOnMaterials` _plane "Color" (`KismetMathLibrary.Conv_LinearColorToVector` _checkpointcolor))
        (`MeshComponent.SetVectorParameterValueOnMaterials` _plane "EmissiveColor" (`KismetMathLibrary.Conv_LinearColorToVector` _checkpointcolor))))))

(fn `UserConstructionScript`)