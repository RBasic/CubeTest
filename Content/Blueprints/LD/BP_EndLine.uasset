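; BP_EndLine is the level finish line, triggered when a BP_BasePlayer overlaps its Box.
; On overlap it activates three fireworks, disables player input, shows the mouse cursor in Game and UI input mode, and adds the WBP_Success widget to the viewport.
; It then plays the ActivateEndline timeline, which drives the Color and EmissiveColor material parameters on the Plane.
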(event `self.Box.OnComponentBeginOverlap`
  (params (OverlappedComponent :type "PrimitiveComponent Object Reference") (OtherActor :type "Actor Object Reference") (OtherComp :type "PrimitiveComponent Object Reference") (OtherBodyIndex :type Integer) (bFromSweep :type Boolean) (SweepResult :type "HitResult Structure (by ref)"))
  (bind _returnvalue (`GameplayStatics.GetPlayerController` 0))
  (bind _plane (`self.Plane`))
  (bind _asbp_base_player (cast `/Game/Blueprints/Player/BP_BasePlayer` OtherActor))
  (set `self.PlayerRef` _asbp_base_player)
  (`ActorComponent.Activate` (`self.Firework`) true)
  (`ActorComponent.Activate` (`self.Firework1`) true)
  (`ActorComponent.Activate` (`self.Firework2`) true)
  (`self.DisableInput` (`self.PlayerRef`) _returnvalue)
  (`WidgetBlueprintLibrary.SetInputMode_GameAndUIEx` _returnvalue null)
  (set `PlayerController.bShowMouseCursor` true _returnvalue)
  (bind _returnvalue_2 (`|CreateWidget` "/Game/Blueprints/UI/WBP_Success.WBP_Success_C" _returnvalue))
  (`UserWidget.AddToViewport` _returnvalue_2 0)
  (bind (_direction _checkpointcolor) (`Timeline|activateEndline`)
    (:`Update`
      (`MeshComponent.SetVectorParameterValueOnMaterials` _plane "Color" (`KismetMathLibrary.Conv_LinearColorToVector` _checkpointcolor))
      (`MeshComponent.SetVectorParameterValueOnMaterials` _plane "EmissiveColor" (`KismetMathLibrary.Conv_LinearColorToVector` _checkpointcolor)))))

(fn `UserConstructionScript`)