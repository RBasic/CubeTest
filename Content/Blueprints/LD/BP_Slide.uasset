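; BP_Slide is a level-design trigger volume that makes players slide while they are inside its Box.
; On begin overlap, it sets Sliding on the BP_BasePlayer and derives SlideVelocity from the normalized movement velocity, keeping X and Y at a fixed speed with zero Z, so entry direction sets the slide.
; On end overlap, it clears the flag and zeroes that velocity, leaving the movement itself to the player Blueprint.
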(event `self.Box.OnComponentBeginOverlap`
  (params (OverlappedComponent :type "PrimitiveComponent Object Reference") (OtherActor :type "Actor Object Reference") (OtherComp :type "PrimitiveComponent Object Reference") (OtherBodyIndex :type Integer) (bFromSweep :type Boolean) (SweepResult :type "HitResult Structure (by ref)"))
  (bind _asbp_base_player (cast `/Game/Blueprints/Player/BP_BasePlayer` OtherActor))
  (set `/Game/Blueprints/Player/BP_BasePlayer.bSliding` true _asbp_base_player)
  (set `/Game/Blueprints/Player/BP_BasePlayer.slideVelocity` (`KismetMathLibrary.MakeVector` (* (.x (`KismetMathLibrary.Normal` (`MovementComponent.Velocity` (`/Game/Blueprints/Player/BP_BasePlayer.FloatingPawnMovement` _asbp_base_player)))) 1000.0) (* (.y (`KismetMathLibrary.Normal` (`MovementComponent.Velocity` (`/Game/Blueprints/Player/BP_BasePlayer.FloatingPawnMovement` _asbp_base_player)))) 1000.0)) _asbp_base_player))

(event `self.Box.OnComponentEndOverlap`
  (params (OverlappedComponent :type "PrimitiveComponent Object Reference") (OtherActor :type "Actor Object Reference") (OtherComp :type "PrimitiveComponent Object Reference") (OtherBodyIndex :type Integer))
  (bind _asbp_base_player (cast `/Game/Blueprints/Player/BP_BasePlayer` OtherActor))
  (set `/Game/Blueprints/Player/BP_BasePlayer.bSliding` false _asbp_base_player)
  (set `/Game/Blueprints/Player/BP_BasePlayer.slideVelocity` (0.0 0.0 0.0) _asbp_base_player))

(fn `UserConstructionScript`)