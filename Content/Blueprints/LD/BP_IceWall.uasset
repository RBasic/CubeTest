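; BP_IceWall is a wall actor that redirects the player's slide when hit.
; On a mesh hit by a BP_BasePlayer, it rotates the movement velocity by a yaw built from the wall's yaw and the travel heading, and writes it to SlideVelocity.
; The heading is approximated by linearly mapping normalized X to an angle, signed by Y.
; A WallHit flag blocks further redirects until a three-second timer calls ResetHit.
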(event `self.StaticMesh.OnComponentHit`
  (params (HitComponent :type "PrimitiveComponent Object Reference") (OtherActor :type "Actor Object Reference") (OtherComp :type "PrimitiveComponent Object Reference") (NormalImpulse :type "Vector Structure") (Hit :type "HitResult Structure (by ref)"))
  (bind (_returnvalue_roll _returnvalue_pitch _returnvalue_yaw) (`KismetMathLibrary.BreakRotator` (`self.K2_GetActorRotation`)))
  (if (not (`self.wallHit`))
    (bind _asbp_base_player (cast `/Game/Blueprints/Player/BP_BasePlayer` OtherActor))
    (bind _velocity (`MovementComponent.Velocity` (`/Game/Blueprints/Player/BP_BasePlayer.FloatingPawnMovement` _asbp_base_player)))
    (bind _returnvalue (* (`KismetMathLibrary.MapRangeClamped` (.x (`KismetMathLibrary.Normal` _velocity)) -1.0 1.0 180.0 0.0) (`KismetMathLibrary.SignOfFloat` (.y (`KismetMathLibrary.Normal` _velocity)))))
    (set `/Game/Blueprints/Player/BP_BasePlayer.slideVelocity` (`KismetMathLibrary.GreaterGreater_VectorRotator` _velocity (`KismetMathLibrary.MakeRotator` 0.0 0.0 (- (- _returnvalue_yaw _returnvalue) _returnvalue))) _asbp_base_player)
    (set `self.wallHit` true)
    (`KismetSystemLibrary.K2_SetTimer` self "ResetHit" 3.0)))

(fn `ResetHit`
  (set `self.wallHit` false))

(fn `UserConstructionScript`)