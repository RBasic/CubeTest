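; BP_Button is a level trigger that toggles or resets a list of linked platforms when a player enters its box.
; Overlap is accepted only from BP_BasePlayer, then calls AnimateBtn and runs TogglePlatform or ResetPlatform on each platform, chosen by the Reset flag.
; AnimateBtn plays one of two timelines, also chosen by Reset, driving the Plane material's color and emissive color as visual feedback.
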(event `AnimateBtn`
  (bind _plane (`self.Plane`))
  (if (`self.Reset`)
    (bind (_direction _checkpointcolor) (`Timeline|activateReset` :!via `PlayFromStart`)
      (:`Update`
        (`MeshComponent.SetVectorParameterValueOnMaterials` _plane "Color" (`KismetMathLibrary.Conv_LinearColorToVector` _checkpointcolor))
        (`MeshComponent.SetVectorParameterValueOnMaterials` _plane "EmissiveColor" (`KismetMathLibrary.Conv_LinearColorToVector` _checkpointcolor))))
    (else
      (bind (_direction_2 _checkpointcolor_2) (`Timeline|activateBtn` :!via `PlayFromStart`)
        (:`Update`
          (`MeshComponent.SetVectorParameterValueOnMaterials` _plane "Color" (`KismetMathLibrary.Conv_LinearColorToVector` _checkpointcolor_2))
          (`MeshComponent.SetVectorParameterValueOnMaterials` _plane "EmissiveColor" (`KismetMathLibrary.Conv_LinearColorToVector` _checkpointcolor_2)))))))

(event `self.Box.OnComponentBeginOverlap`
  (params (OverlappedComponent :type "PrimitiveComponent Object Reference") (OtherActor :type "Actor Object Reference") (OtherComp :type "PrimitiveComponent Object Reference") (OtherBodyIndex :type Integer) (bFromSweep :type Boolean) (SweepResult :type "HitResult Structure (by ref)"))
  (cast `/Game/Blueprints/Player/BP_BasePlayer` OtherActor)
  (`self.AnimateBtn`)
  (for _array_element (`self.Platforms`)
    (if (`self.Reset`)
      (`/Game/Blueprints/LD/BP_PlatformEnigma.ResetPlatform` _array_element)
      (else
        (`/Game/Blueprints/LD/BP_PlatformEnigma.TogglePlatform` _array_element)))))

(fn `UserConstructionScript`)