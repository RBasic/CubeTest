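; Level-design actor that builds a track by repeating a static mesh along its spline.
; The construction script calls GenerateTrack, which adds one spline mesh component per section, using SectionLength multiplied by actor X scale.
; Each piece gets the configured mesh, material, physical material, scale and forward axis.
; Start and end points follow the spline, with tangents clamped to section length and spline roll applied for banking.
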(fn `GenerateTrack`
  (params (staticMesh :type "StaticMesh Object Reference") (meshMaterial :type "MaterialInstance Object Reference") (physicalMat :type "PhysicalMaterial Object Reference") (scale :type "Vector Structure") (orientation :type "ESplineMeshAxis Enum" :default "X"))
  (bind _returnvalue_x (`KismetMathLibrary.BreakVector` (`self.GetActorScale3D`)))
  (bind _spline (`self.Spline`))
  (bind _sectionlength (`self.SectionLength`))
  (bind _sectionlength_2 (`self.SectionLength`))
  (set `self.SectionLength` (* _returnvalue_x _sectionlength))
  (for _index (range (+ (`KismetMathLibrary.FTrunc` (/ (`SplineComponent.GetSplineLength` (`self.Spline`)) _sectionlength)) 1))
    (bind _returnvalue (`AddComponent|NODE_AddSplineMeshComponent-0`))
    (`StaticMeshComponent.SetStaticMesh` _returnvalue staticMesh)
    (`PrimitiveComponent.SetMaterial` _returnvalue 0 meshMaterial)
    (`SplineMeshComponent.SetForwardAxis` _returnvalue orientation true)
    (`SceneComponent.SetRelativeScale3D` _returnvalue scale)
    (`PrimitiveComponent.SetPhysMaterialOverride` _returnvalue physicalMat)
    (bind _returnvalue_2 (* _index _sectionlength_2))
    (bind _returnvalue_3 (* (+ _index 1) _sectionlength_2))
    (`SplineMeshComponent.SetStartAndEnd` _returnvalue (`SplineComponent.GetLocationAtDistanceAlongSpline` _spline _returnvalue_2 "Local") (`KismetMathLibrary.ClampVectorSize` (`SplineComponent.GetTangentAtDistanceAlongSpline` _spline _returnvalue_2 "Local") 0.0 (`self.SectionLength`)) (`SplineComponent.GetLocationAtDistanceAlongSpline` _spline _returnvalue_3 "Local") (`KismetMathLibrary.ClampVectorSize` (`SplineComponent.GetTangentAtDistanceAlongSpline` _spline _returnvalue_3 "Local") 0.0 (`self.SectionLength`)) true)
    (`SplineMeshComponent.SetStartRoll` _returnvalue (`KismetMathLibrary.DegreesToRadians` (`SplineComponent.GetRollAtDistanceAlongSpline` _spline _returnvalue_2 "Local")) true)
    (`SplineMeshComponent.SetEndRoll` _returnvalue (`KismetMathLibrary.DegreesToRadians` (`SplineComponent.GetRollAtDistanceAlongSpline` _spline _returnvalue_3 "Local")) true)))

(fn `UserConstructionScript`
  (`self.GenerateTrack` (`self.Static Mesh`) (`self.Mesh Material`) (`self.Physical Mat`) (`self.Scale`) (`self.Orientation`)))