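; BP_CustomGameMode is a game mode Blueprint that keeps an elapsed-seconds counter for the game.
; StartGameTimer optionally resets Timer, then starts a looping one-second timer, bound by function name, that calls HandleTimer to increment it.
; StopGameTimer clears and invalidates the stored timer handle, and nothing in the graph starts the timer automatically.
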(event `StartGameTimer`
  (params (Reset :type Boolean))
  (if Reset
    (set `self.Timer` 0))
  (bind _returnvalue (`KismetSystemLibrary.K2_SetTimer` self "HandleTimer" 1.0 true))
  (set `self.TimerHandler` _returnvalue))

(event `StopGameTimer`
  (`KismetSystemLibrary.K2_ClearAndInvalidateTimerHandle` (`self.TimerHandler`)))

(fn `HandleTimer`
  (`/Engine/EditorBlueprintResources/StandardMacros.IncrementInt` (`self.Timer`)))

(fn `UserConstructionScript`)