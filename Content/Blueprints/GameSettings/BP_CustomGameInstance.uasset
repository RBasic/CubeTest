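; Custom game instance that owns level progression save data: each level's availability and high score.
; LoadSaveData loads the BP_SaveLevels slot, or creates and saves a new object if none exists, and caches it.
; SaveLevelsData optionally updates the current level's high score, unlocks the next level and writes to the slot.
; Saving and GetCurrentLevelData derive the array index from a single digit at character index 3 of the level name.
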(fn `GetCurrentLevelData`
  (returns (levelData :type "/Game/Blueprints/Structures/Struct_LevelAvailability Structure"))
  (bind _returnvalue (`GameplayStatics.GetCurrentLevelName` true))
  (return (`|GetArrayItem` (`/Game/Blueprints/GameSettings/BP_SaveLevels.levelsAvailability` (`self.SaveLevels`)) (- (`KismetStringLibrary.Conv_StringToInt` (`KismetStringLibrary.GetSubstring` _returnvalue 3)) 1))))

(fn `LoadSaveData`
  (returns (SaveLevels :type "/Game/Blueprints/GameSettings/BP_SaveLevels Object Reference"))
  (bind _returnvalue (`GameplayStatics.DoesSaveGameExist` (`self.SaveLevelsSlot`)))
  (if _returnvalue
    (bind _returnvalue_2 (`GameplayStatics.LoadGameFromSlot` (`self.SaveLevelsSlot`)))
    (bind _asbp_save_levels (cast `/Game/Blueprints/GameSettings/BP_SaveLevels` _returnvalue_2))
    (set `self.SaveLevels` _asbp_save_levels)
    (else
      (bind _returnvalue_3 (`GameplayStatics.CreateSaveGameObject` "/Game/Blueprints/GameSettings/BP_SaveLevels.BP_SaveLevels_C"))
      (bind _output_get (set `self.SaveLevels` _returnvalue_3))
      (`GameplayStatics.SaveGameToSlot` _output_get (`self.SaveLevelsSlot`))))
  (return (`self.SaveLevels`)))

(fn `SaveLevelsData`
  (params (NewHighScore :type Boolean) (HighScore :type Integer))
  (bind _levelsavailability (`/Game/Blueprints/GameSettings/BP_SaveLevels.levelsAvailability` (`self.SaveLevels`)))
  (bind _returnvalue (`GameplayStatics.GetCurrentLevelName` true))
  (bind _returnvalue_2 (`KismetStringLibrary.Conv_StringToInt` (`KismetStringLibrary.GetSubstring` _returnvalue 3)))
  (bind _returnvalue_3 (- _returnvalue_2 1))
  (bind (_output_levelname _output_isavailable _output_levelbtntext _output_highscore) (break `/Game/Blueprints/Structures/Struct_LevelAvailability` (`|GetArrayItem` _levelsavailability _returnvalue_3)))
  (`KismetArrayLibrary.Array_Set` _levelsavailability _returnvalue_3 (make `/Game/Blueprints/Structures/Struct_LevelAvailability` _output_levelname _output_isavailable _output_levelbtntext (select `bool` NewHighScore :`false` _output_highscore :`true` HighScore)))
  (bind (_output_levelname_2 _output_isavailable_2 _output_levelbtntext_2 _output_highscore_2) (break `/Game/Blueprints/Structures/Struct_LevelAvailability` (`|GetArrayItem` _levelsavailability _returnvalue_2)))
  (`KismetArrayLibrary.Array_Set` _levelsavailability _returnvalue_2 (make `/Game/Blueprints/Structures/Struct_LevelAvailability` _output_levelname_2 true _output_levelbtntext_2 _output_highscore_2))
  (`GameplayStatics.SaveGameToSlot` (`self.SaveLevels`) (`self.SaveLevelsSlot`)))